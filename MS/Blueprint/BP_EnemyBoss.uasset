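; Boss enemy actor that chases BP_Player and displays its health through a WBP_EnemyHP widget.
; BeginPlay initializes HP and finds the player; Tick moves straight toward it without sweep, snaps rotation to face it, then interpolates the whole actor's rotation toward the camera.
; MyApplyDamage subtracts HP, refreshes the widget and returns remaining HP.
; DropItem spawns BP_Treasure at a given location; neither function is called here.
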(event EventBeginPlay
  ;[1 1 1] EnemyHp초기화 & 플레이어 찾기
  (Variables|Default|SetCurrentHP (Variables|Default|GetEnemyHP))
  (Utilities|IsValid (Variables|Default|GetTarget)
    (:Is%20Not%20Valid
      (bind _returnvalue (Actor|GetActorOfClass "/Game/EB/Blueprints/BP_Player.BP_Player_C")) ; 현재 레벨에 있는 액터 찾기
      (Variables|Default|SetTarget _returnvalue)
      (CallFunction|UpdateHPUI))))

(event EventTick
  (params (DeltaSeconds :type Float%20%28single-precision%29))
  ;[1 1 1] 플레이어를 향해 이동 & 체력 UI 카메라를 바라보는 방향으로 회전
  (Transformation|SetActorLocation (+ (Transformation|GetActorLocation) (* (Math|Vector|Normalize (- (Transformation|GetActorLocation (Variables|Default|GetTarget)) (Transformation|GetActorLocation))) (Variables|Default|GetSpeed) (Utilities|Time|GetWorldDeltaSeconds))) false false)
  ;;[1 1 1] 플레이어 바라보는 방향으로 회전
  (Transformation|SetActorRotation (Math|Rotator|FindLookatRotation (Transformation|GetActorLocation) (Transformation|GetActorLocation (Variables|Default|GetTarget))))
  (Transformation|SetActorRotation (Math|Interpolation|RInterpTo (Transformation|GetActorRotation) (Math|Rotator|FindLookatRotation (Transformation|GetActorLocation) (Transformation|GetActorLocation (Game|GetPlayerCameraManager 0))) (Utilities|Time|GetWorldDeltaSeconds) 5.0)))

(fn ConstructionScript)

(fn MyApplyDamage
  (params (Power :type Integer))
  (Variables|Default|SetCurrentHP (- (Variables|Default|GetCurrentHP) Power))
  (CallFunction|UpdateHPUI)
  (return (Variables|Default|GetCurrentHP)))

(fn DropItem
  (params (Location :type Vector))
  (Game|SpawnActorfromClass "/Game/MS/Blueprint/BP_Treasure.BP_Treasure_C" (Math|Transform|MakeTransform Location "0, 0, 0" "1.000000,1.000000,1.000000") "Undefined" "MultiplyWithRoot" 0 0)
  (return))

(fn UpdateHPUI
  (bind _aswbp_enemy_hp (Utilities|Casting|CastToWBP_EnemyHP (UserInterface|GetWidget (Variables|Default|GetWidgetHP))))
  (Default|SetHP _aswbp_enemy_hp (Variables|Default|GetCurrentHP)))