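; BP_Treasure is a treasure actor that opens a treasure screen when the player touches it.
; On overlap with BP_Player it pauses the game, adds a WBP_Treasure widget to the viewport, shows the mouse cursor and resets CurrentTime to zero.
; A coin-burst Niagara effect with a delay and a UI-only input switch are present but unconnected, so they never run.
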(event EventBeginPlay)

(event Collision|EventActorBeginOverlap
  (params (OtherActor :type Actor%20Object%20Reference))
  (Utilities|Casting|CastToBP_Player OtherActor)
  (Game|SetGamePaused true)
  (bind _returnvalue (UserInterface|CreateWidget "/Game/MS/UI/WBP_Treasure.WBP_Treasure_C"))
  (UserInterface|Viewport|AddtoViewport _returnvalue 0)
  (Variables|/Script/Engine.PlayerController|SetbShowMouseCursor (Game|GetPlayerController 0) true) ; 마우스 커서 보이기
  (Variables|Default|SetcurrentTime 0.0))

(event EventTick
  (params (DeltaSeconds :type Float%20%28single-precision%29)))

(fn ConstructionScript)