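; BP_Enemy2 is an enemy actor that chases BP_Player and shows its health in a widget.
; BeginPlay sets HP and finds the target; Tick moves toward it without sweep, snaps rotation to face it, then interpolates toward the camera.
; MyApplyDamage subtracts HP and updates the widget, while DropItem spawns a BP_GaugeItem; neither is called here.
; Widget-rotation and paused level-up screen logic remain disconnected.
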(event EventBeginPlay
  (Variables|Default|SetCurrentHP (Variables|Default|GetEnemyHP))
  (Utilities|IsValid (Variables|Default|GetTarget)
    (:Is%20Not%20Valid
      (bind _returnvalue (Actor|GetActorOfClass "/Game/EB/Blueprints/BP_Player.BP_Player_C")) ; 현재 레벨에 있는 액터 찾기
      (Variables|Default|SetTarget _returnvalue)
      (CallFunction|UpdateHPUI))))

(event EventTick
  (params (DeltaSeconds :type Float%20%28single-precision%29))
  (Utilities|FlowControl|Sequence
    (:then_0
      (Transformation|SetActorLocation (+ (Transformation|GetActorLocation) (* (Math|Vector|Normalize (- (Transformation|GetActorLocation (Variables|Default|GetTarget)) (Transformation|GetActorLocation))) (Variables|Default|GetSpeed) (Utilities|Time|GetWorldDeltaSeconds))) false false)
      ;[1 1 1] 플레이어 바라보는 방향으로 회전
      (Transformation|SetActorRotation (Math|Rotator|FindLookatRotation (Transformation|GetActorLocation) (Transformation|GetActorLocation (Variables|Default|GetTarget))))
      (Transformation|SetActorRotation (Math|Interpolation|RInterpTo (Transformation|GetActorRotation) (Math|Rotator|FindLookatRotation (Transformation|GetActorLocation) (Transformation|GetActorLocation (Game|GetPlayerCameraManager 0))) (Utilities|Time|GetWorldDeltaSeconds) 5.0)))))

(fn ConstructionScript)

(fn MyApplyDamage
  (params (power :type Integer))
  (Variables|Default|SetCurrentHP (- (Variables|Default|GetCurrentHP) power))
  (bind _aswbp_enemy_hp (Utilities|Casting|CastToWBP_EnemyHP (UserInterface|GetWidget (Variables|Default|GetWidgetHP))))
  (Default|SetHP _aswbp_enemy_hp (Variables|Default|GetCurrentHP))
  (Development|PrintText (Utilities|Text|ToText(Integer) (Variables|Default|GetCurrentHP)))
  (return (Variables|Default|GetCurrentHP)))

(fn DropItem
  (params (Location :type Vector))
  (Game|SpawnActorfromClass "/Game/EB/Blueprints/BP_GaugeItem.BP_GaugeItem_C" (Math|Transform|MakeTransform Location "0, 0, 0" "1.000000,1.000000,1.000000") "Undefined" "MultiplyWithRoot" 0 0)
  (return))

(fn UpdateHPUI
  (bind _aswbp_enemy_hp (Utilities|Casting|CastToWBP_EnemyHP (UserInterface|GetWidget (Variables|Default|GetWidgetHP))))
  (Default|SetHP _aswbp_enemy_hp (Variables|Default|GetCurrentHP)))