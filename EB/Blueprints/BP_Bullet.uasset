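; BP_Bullet is a projectile that damages BP_Enemy, BP_Enemy2 and BP_EnemyBoss on overlap.
; It moves along its forward vector each tick through a swept, delta-time-scaled Translate function.
; Each hit casts per enemy type, spawns an explosion and calls MyApplyDamage with Power, or BossPower for the boss.
; At zero or lower returned value, the enemy drops an item, and both actors are destroyed; otherwise the bullet persists.
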(event Collision|EventActorBeginOverlap
  (params (OtherActor :type Actor%20Object%20Reference))
  ;[1 1 1] Enemy와 충돌 시 enemyHP가 0보다 작거나 같을 시  drop item후 Destroy
  (Utilities|FlowControl|Sequence
    (:then_0
      ;;[1 1 1] Enemy 1
      (bind _asbp_enemy (Utilities|Casting|CastToBP_Enemy OtherActor))
      (Effects|SpawnEmitteratLocation "/Game/StarterContent/Particles/P_Explosion.P_Explosion" (Transformation|GetActorLocation _asbp_enemy))
      (bind _resulthp (Default|MyApplyDamage _asbp_enemy (Variables|Default|GetPower)))
      (if (<= _resulthp 0)
        (Default|DropItem _asbp_enemy (Transformation|GetActorLocation _asbp_enemy))
        (Actor|DestroyActor _asbp_enemy)
        (Actor|DestroyActor)))
    (:then_1
      ;;[1 1 1] Enemy2
      (bind _asbp_enemy_2 (Utilities|Casting|CastToBP_Enemy2 OtherActor))
      (Effects|SpawnEmitteratLocation "/Game/StarterContent/Particles/P_Explosion.P_Explosion" (Transformation|GetActorLocation _asbp_enemy_2))
      (bind _resulthp_2 (Default|MyApplyDamage _asbp_enemy_2 (Variables|Default|GetPower)))
      (if (<= _resulthp_2 0)
        (Default|DropItem _asbp_enemy_2 (Transformation|GetActorLocation _asbp_enemy_2))
        (Actor|DestroyActor _asbp_enemy_2)
        (Actor|DestroyActor)))
    (:then_2
      ;;[1 1 1] Boss Enemy
      (bind _asbp_enemy_boss (Utilities|Casting|CastToBP_EnemyBoss OtherActor))
      ;;;[1 1 1] rh공격시 이펙트 다운받기
      (Effects|SpawnEmitteratLocation "/Game/StarterContent/Particles/P_Explosion.P_Explosion" (Transformation|GetActorLocation _asbp_enemy_boss))
      (bind _resulthp_3 (Default|MyApplyDamage _asbp_enemy_boss (Variables|Default|GetBossPower)))
      (if (<= _resulthp_3 0)
        (Default|DropItem _asbp_enemy_boss (Transformation|GetActorLocation _asbp_enemy_boss))
        (Actor|DestroyActor _asbp_enemy_boss)
        (Actor|DestroyActor)))))

(event EventTick
  (params (DeltaSeconds :type Float%20%28single-precision%29))
  ;[1 1 1] 총알 이동
  (CallFunction|Translate (Transformation|GetActorForwardVector) (Variables|Default|GetSpeed)))

(fn ConstructionScript)

(fn Translate
  (params (Direction :type Vector) (Speed :type Float%20%28double-precision%29))
  ;[1 1 1] P = P0 + velocity(dir*speed)*deltaSecond
  (Transformation|SetActorLocation (+ (Transformation|GetActorLocation) (* Direction Speed (Utilities|Time|GetWorldDeltaSeconds))) true false))