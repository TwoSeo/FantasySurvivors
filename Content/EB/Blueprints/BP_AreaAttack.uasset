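; BP_AreaAttack is an area attack actor that follows a target, defaulting to BP_Player, and periodically damages an overlapping BP_Enemy.
; Tick moves it toward the target in X and Y at a set speed.
; Overlap stores the enemy in a single variable and starts a looping AutoHit timer, paused when an enemy leaves.
; AutoHit applies Power as damage, then triggers an item drop and destroys the enemy at zero HP.
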(event Custom|AutoHit
  ;[1 1 1] 공격
  (Utilities|IsValid (stale Collision|EventActorBeginOverlap _asbp_enemy)
    (:Is%20Valid
      (Default|MyApplyDamage (stale Collision|EventActorBeginOverlap _asbp_enemy) (Variables|Default|GetPower))
      ;;[1 1 1] Enemy HP가 0이라면
      (if (== (Variables|/Game/EB/Blueprints/BP_Enemy.BP_Enemy_C|GetCurrentHP (stale Collision|EventActorBeginOverlap _asbp_enemy)) 0)
        ;;[1 1 1] 아이템 드롭 후 죽음
        (Default|DropItem (stale Collision|EventActorBeginOverlap _asbp_enemy) (Transformation|GetActorLocation (stale Collision|EventActorBeginOverlap _asbp_enemy)))
        (Actor|DestroyActor (stale Collision|EventActorBeginOverlap _asbp_enemy))))))

(event Collision|EventActorBeginOverlap
  (params (OtherActor :type Actor%20Object%20Reference))
  ;[1 1 1] 공격
  ;;[1 1 1] Area Attack과 Enemy가 충돌 했을 때
  (bind _asbp_enemy (Utilities|Casting|CastToBP_Enemy OtherActor))
  ;;[1 1 1] 적의 공격력이 0이 될때까지 반복
  (bind _returnvalue (Utilities|Time|SetTimerbyEvent (delegate Custom|AutoHit) (Variables|Default|GetAttackTime) true)))

(event EventTick
  (params (DeltaSeconds :type Float%20%28single-precision%29))
  (bind _returnvalue (Transformation|GetActorLocation))
  (bind _returnvalue_2 (Transformation|GetActorLocation))
  (bind _returnvalue_3 (Utilities|Time|GetWorldDeltaSeconds))
  (bind _target (Variables|Default|GetTarget))
  (bind _speed (Variables|Default|Getspeed))
  (bind _returnvalue_4 (Transformation|GetActorLocation _target))
  (bind _returnvalue_5 (- _returnvalue_4 _returnvalue_2))
  (bind _returnvalue_6 (Math|Vector|Normalize _returnvalue_5))
  (bind _returnvalue_7 (* _returnvalue_6 _speed _returnvalue_3))
  (bind _returnvalue_8 (+ (Math|Vector|MakeVector (.x _returnvalue) (.y _returnvalue) 0.0) _returnvalue_7))
  ;[1 1 1] 살아가면서 목적지를 향해 계속 이동
  (Transformation|SetActorLocation (Math|Vector|MakeVector (.x _returnvalue_8) (.y _returnvalue_8) 0.0) false false))

(event EventBeginPlay
  ;[1 1 1] 태어날 때 목적지가 유효하지 않다면주인공 플레이어를 목적지로 설정
  (Utilities|IsValid (Variables|Default|GetTarget)
    (:Is%20Not%20Valid
      (bind _returnvalue (Actor|GetActorOfClass "/Game/EB/Blueprints/BP_Player.BP_Player_C"))
      (bind _output_get (Variables|Default|SetTarget _returnvalue))
      (Development|PrintString (Utilities|GetDisplayName _output_get)))))

(event Collision|EventActorEndOverlap
  (params (OtherActor :type Actor%20Object%20Reference))
  ;[1 1 1] 공격
  ;;[1 1 1] 충돌이 끝났을 때 timer 멈춤
  (Utilities|Casting|CastToBP_Enemy OtherActor)
  (Utilities|Time|PauseTimerbyHandle (stale Collision|EventActorBeginOverlap _returnvalue)))

(fn ConstructionScript)