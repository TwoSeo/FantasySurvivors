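; Game mode for a Fantasy Survivors level that runs a three-minute survival round.
; On BeginPlay it shows the in-game HUD widget and starts a looping timer that spawns HP pickups at random points in a square area around the player.
; When the delay ends it shows the game-clear widget, pauses the game, switches to UI-only input with a visible cursor and plays a clear sound.
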(event Custom|SpawnHPItem
  (bind _returnvalue (Game|Player|GetPlayerPawn 0))
  (bind _returnvalue_2 (Transformation|GetActorLocation _returnvalue))
  ;[1 1 1] Item Random Spawn
  (Game|SpawnActorfromClass "/Game/EB/Blueprints/BP_HP.BP_HP_C" (Math|Transform|MakeTransform (Math|Vector|MakeVector (Math|Random|RandomFloatinRange (- (.x _returnvalue_2) 1e+03) (+ (.x _returnvalue_2) 1e+03)) (Math|Random|RandomFloatinRange (- (.y _returnvalue_2) 1e+03) (+ (.y _returnvalue_2) 1e+03)) 5.0) "0, 0, 0" "1.000000,1.000000,1.000000") "Undefined" "MultiplyWithRoot" 0 0))

(event EventBeginPlay
  (bind _returnvalue (Game|GetPlayerController 0))
  (Utilities|FlowControl|Sequence
    (:then_0
      ;[1 1 1] 시작되면 UI Show
      (bind _returnvalue_2 (UserInterface|CreateWidget "/Game/EB/UI/WBP_InGame.WBP_InGame_C"))
      (UserInterface|Viewport|AddtoViewport _returnvalue_2 10))
    (:then_1
      ;[1 1 1] 주기
      (Utilities|Time|SetTimerbyEvent (delegate Custom|SpawnHPItem) (Variables|Default|GetHPItemSpawnTime) true))
    (:then_2
      (Utilities|FlowControl|Delay 1.8e+02)
      (bind _returnvalue_3 (UserInterface|CreateWidget "/Game/EB/UI/WBP_GameClear.WBP_GameClear_C"))
      (UserInterface|Viewport|AddtoViewport _returnvalue_3 10)
      (Game|SetGamePaused true)
      (Variables|/Script/Engine.PlayerController|SetbShowMouseCursor _returnvalue true) ; 마우스 커서 보이기
      (Input|SetInputModeUIOnly _returnvalue 0 "DoNotLock" false)
      (Audio|PlaySound2D "/Game/EB/Sounds/LevelClear.LevelClear" 1.0 1.0 0.0 0 0))))

(fn ConstructionScript)