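; BP_GaugeItem is a pickup that fills the player's gauge and drives leveling up.
; On overlap with BP_Player, a looping timer pulls it toward Target (the player by default) at fixed height.
; After a short delay it adds to Gauge and destroys itself.
; When Gauge exactly equals MaxGauge, it resets Gauge, increments PlayerLevel, pauses the game and shows WBP_LevelUP with the mouse cursor.
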(event Custom|EatGargeItem
  (bind _returnvalue (Transformation|GetActorLocation))
  (bind _returnvalue_2 (Transformation|GetActorLocation))
  (bind _returnvalue_3 (Utilities|Time|GetWorldDeltaSeconds))
  (bind _target (Variables|Default|GetTarget))
  (bind _speed (Variables|Default|Getspeed))
  (bind _returnvalue_4 (Transformation|GetActorLocation _target))
  (bind _returnvalue_5 (- _returnvalue_4 _returnvalue_2))
  (bind _returnvalue_6 (Math|Vector|Normalize _returnvalue_5))
  (bind _returnvalue_7 (* _returnvalue_6 _speed _returnvalue_3))
  (bind _returnvalue_8 (+ (Math|Vector|MakeVector (.x _returnvalue) (.y _returnvalue) 0.0) _returnvalue_7))
  ;[1 1 1] 살아가면서 목적지를 향해 계속 이동
  (Transformation|SetActorLocation (Math|Vector|MakeVector (.x _returnvalue_8) (.y _returnvalue_8) 3e+01) false false))

(event Collision|EventActorBeginOverlap
  (params (OtherActor :type Actor%20Object%20Reference))
  ;[1 1 1] Gauge Item Player에 적용
  (bind _asbp_player (Utilities|Casting|CastToBP_Player OtherActor))
  (Utilities|Time|SetTimerbyEvent (delegate Custom|EatGargeItem) 0.1 true)
  (Utilities|FlowControl|Delay 0.15)
  ;;[1 1 1] Item Get -> Gauge+
  (bind _output_get (Variables|/Game/EB/Blueprints/BP_Player.BP_Player_C|SetGauge _asbp_player (+ (Variables|/Game/EB/Blueprints/BP_Player.BP_Player_C|GetGauge _asbp_player) (Variables|Default|GetPlusGauge))))
  (Actor|DestroyActor)
  ;;[1 1 1] Gauge=MaxGauge-> reset/ LevelUP
  (if (== _output_get (Variables|/Game/EB/Blueprints/BP_Player.BP_Player_C|GetMaxGauge _asbp_player))
    (Variables|/Game/EB/Blueprints/BP_Player.BP_Player_C|SetGauge _asbp_player 0)
    (Math|Integer|IncrementInt (Variables|/Game/EB/Blueprints/BP_Player.BP_Player_C|GetPlayerLevel _asbp_player)
      (:%20%20
        (Development|PrintString "Level UP!!")
        (Game|SetGamePaused true)
        (bind _returnvalue (UserInterface|CreateWidget "/Game/MS/UI/WBP_LevelUP.WBP_LevelUP_C"))
        (UserInterface|Viewport|AddtoViewport _returnvalue 0)
        (Variables|/Script/Engine.PlayerController|SetbShowMouseCursor (Game|GetPlayerController 0) true) ; 마우스 커서 보이기
      ))))

(event EventBeginPlay
  ;[1 1 1] 태어날 때 목적지가 유효하지 않다면주인공 플레이어를 목적지로 설정
  (Utilities|IsValid (Variables|Default|GetTarget)
    (:Is%20Not%20Valid
      (bind _returnvalue (Actor|GetActorOfClass "/Game/EB/Blueprints/BP_Player.BP_Player_C"))
      (bind _output_get (Variables|Default|SetTarget _returnvalue))
      (Development|PrintString (Utilities|GetDisplayName _output_get)))))

(fn ConstructionScript)