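; BP_Bullet is a projectile that damages BP_Enemy actors on overlap.
; Each tick, Translate moves it along its forward vector at Speed, scaled by delta time, using a swept move.
; On overlap with an enemy it spawns an explosion and calls MyApplyDamage with Power.
; If the returned value is zero or less, the enemy drops an item and both actors are destroyed; otherwise the bullet keeps flying.
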(event Collision|EventActorBeginOverlap
  (params (OtherActor :type Actor%20Object%20Reference))
  (bind _asbp_enemy (Utilities|Casting|CastToBP_Enemy OtherActor))
  (Effects|SpawnEmitteratLocation "/Game/StarterContent/Particles/P_Explosion.P_Explosion" (Transformation|GetActorLocation _asbp_enemy))
  (bind _resulthp (Default|MyApplyDamage _asbp_enemy (Variables|Default|GetPower)))
  (if (<= _resulthp 0)
    (Default|DropItem _asbp_enemy (Transformation|GetActorLocation _asbp_enemy))
    (Actor|DestroyActor _asbp_enemy)
    (Actor|DestroyActor)))

(event EventTick
  (params (DeltaSeconds :type Float%20%28single-precision%29))
  (CallFunction|Translate (Transformation|GetActorForwardVector) (Variables|Default|GetSpeed)))

(fn ConstructionScript)

(fn Translate
  (params (Direction :type Vector) (Speed :type Float%20%28double-precision%29))
  ;[1 1 1] P = P0 + velocity(dir*speed)*deltaSecond
  (Transformation|SetActorLocation (+ (Transformation|GetActorLocation) (* Direction Speed (Utilities|Time|GetWorldDeltaSeconds))) true false))