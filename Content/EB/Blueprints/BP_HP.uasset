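; BP_HP is an actor that explodes when a BP_Bullet overlaps it.
; On BeginPlay it defaults an invalid Target to the BP_Player actor and prints that name, though these graphs do not use Target further.
; AddExplosion plays the Rock sound in 2D, spawns BP_Explosion and a smoke emitter at its location, then destroys the actor.
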(event Collision|EventActorBeginOverlap
  (params (OtherActor :type Actor%20Object%20Reference))
  (Utilities|Casting|CastToBP_Bullet OtherActor)
  (CallFunction|AddExplosion))

(event EventBeginPlay
  ;[1 1 1] 태어날 때 목적지가 유효하지 않다면주인공 플레이어를 목적지로 설정
  (Utilities|IsValid (Variables|Default|GetTarget)
    (:Is%20Not%20Valid
      (bind _returnvalue (Actor|GetActorOfClass "/Game/EB/Blueprints/BP_Player.BP_Player_C"))
      (bind _output_get (Variables|Default|SetTarget _returnvalue))
      (Development|PrintString (Utilities|GetDisplayName _output_get)))))

(fn ConstructionScript)

(fn AddExplosion
  (bind _returnvalue (Transformation|GetActorLocation))
  (Audio|PlaySound2D "/Game/EB/Sounds/Rock.Rock" 1.0 1.0 0.0 0 0)
  (Game|SpawnActorfromClass "/Game/EB/Blueprints/BP_Explosion.BP_Explosion_C" (Math|Transform|MakeTransform _returnvalue "0, 0, 0" "1.000000,1.000000,1.000000") "Undefined" "MultiplyWithRoot" 0 0)
  (Effects|SpawnEmitteratLocation "/Game/StarterContent/Particles/P_Smoke.P_Smoke" _returnvalue)
  (Actor|DestroyActor))