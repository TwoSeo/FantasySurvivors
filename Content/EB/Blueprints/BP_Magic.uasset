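; BP_Magic is a homing magic projectile that damages enemies it overlaps.
; On BeginPlay it homes ProjectileMovement onto the closest "Enemy"-tagged actor within the initial ClosestDistance, self-destructing after a delay once targeted.
; Overlapping BP_Enemy, BP_Enemy2 or BP_EnemyBoss spawns an explosion, applies Power damage and destroys the projectile.
; Kills trigger item drop, BP_Player's kill count and enemy death, plus a roar for Enemy2 and Boss.
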(event EventBeginPlay
  (bind _projectilemovement (Variables|Default|GetProjectileMovement))
  ;[1 1 1] 생성된 적 중 가장 가까운 목적지 설정
  (bind _outactors (Actor|GetAllActorswithTag "Enemy")) ; Enemy라는 태그가 있는 적 탐색
  (for _array_element _outactors
    (if (< (Math|Vector|VectorLength (- (Transformation|GetActorLocation) (Transformation|GetWorldLocation (Variables|/Script/Engine.Actor|GetRootComponent _array_element)))) (Variables|Default|GetClosestDistance))
      (Variables|Default|SetClosestDistance (Math|Vector|VectorLength (- (Transformation|GetActorLocation) (Transformation|GetWorldLocation (Variables|/Script/Engine.Actor|GetRootComponent _array_element)))))
      (Variables|/Script/Engine.ProjectileMovementComponent|SetHomingTargetComponent _projectilemovement (Variables|/Script/Engine.Actor|GetRootComponent _array_element))
      (Variables|/Script/Engine.ProjectileMovementComponent|SetbIsHomingProjectile _projectilemovement true)
      (Variables|/Script/Engine.ProjectileMovementComponent|SetHomingAccelerationMagnitude _projectilemovement 1e+04)
      (Utilities|FlowControl|Delay 2.0)
      (Actor|DestroyActor))))

(event EventTick
  (params (DeltaSeconds :type Float%20%28single-precision%29)))

(event Collision|EventActorBeginOverlap
  (params (OtherActor :type Actor%20Object%20Reference))
  (Utilities|FlowControl|Sequence
    (:then_0
      (bind _asbp_enemy (Utilities|Casting|CastToBP_Enemy OtherActor))
      ;[1 1 1] 충돌 효과
      (Effects|SpawnEmitteratLocation "/Game/StarterContent/Particles/P_Explosion.P_Explosion" (Transformation|GetActorLocation))
      ;[1 1 1] Enemy Damage
      (bind _resulthp (Default|MyApplyDamage _asbp_enemy (Variables|Default|GetPower)))
      (if (<= _resulthp 0)
        (Default|DropItem _asbp_enemy (Transformation|GetActorLocation _asbp_enemy))
        (bind _returnvalue (Actor|GetActorOfClass "/Game/EB/Blueprints/BP_Player.BP_Player_C"))
        (Default|CountKill _returnvalue _returnvalue)
        (Variables|/Game/EB/Blueprints/BP_Enemy.BP_Enemy_C|SetIsDead _asbp_enemy true)
        (Default|EnemyDeath _asbp_enemy (Transformation|GetActorLocation _asbp_enemy))
        (Actor|DestroyActor)
        (else
          (Actor|DestroyActor))))
    (:then_1
      (bind _asbp_enemy_2 (Utilities|Casting|CastToBP_Enemy2 OtherActor))
      ;[1 1 1] 충돌 효과
      (Effects|SpawnEmitteratLocation "/Game/StarterContent/Particles/P_Explosion.P_Explosion" (Transformation|GetActorLocation))
      (bind _resulthp_2 (Default|MyApplyDamage _asbp_enemy_2 (Variables|Default|GetPower)))
      (if (<= _resulthp_2 0)
        (Default|DropItem _asbp_enemy_2 (Transformation|GetActorLocation _asbp_enemy_2))
        (bind _returnvalue_2 (Actor|GetActorOfClass "/Game/EB/Blueprints/BP_Player.BP_Player_C"))
        (Default|CountKill _returnvalue_2 _returnvalue_2)
        (Variables|/Game/EB/Blueprints/BP_Enemy2.BP_Enemy2_C|SetIsDead _asbp_enemy_2 true)
        (Default|EnemyDeath _asbp_enemy_2 (Transformation|GetActorLocation _asbp_enemy_2))
        (Audio|PlaySound2D "/Game/MS/Sound/monster-roar-131214.monster-roar-131214" 0.2 1.0 0.0 0 0)
        (Actor|DestroyActor)
        (else
          (Actor|DestroyActor))))
    (:then_2
      (bind _asbp_enemy_boss (Utilities|Casting|CastToBP_EnemyBoss OtherActor))
      ;[1 1 1] 충돌 효과
      (Effects|SpawnEmitteratLocation "/Game/StarterContent/Particles/P_Explosion.P_Explosion" (Transformation|GetActorLocation))
      (bind _resulthp_3 (Default|MyApplyDamage _asbp_enemy_boss (Variables|Default|GetPower)))
      (if (<= _resulthp_3 0)
        (Default|DropItem _asbp_enemy_boss (Transformation|GetActorLocation _asbp_enemy_boss))
        (bind _returnvalue_3 (Actor|GetActorOfClass "/Game/EB/Blueprints/BP_Player.BP_Player_C"))
        (Default|CountKill _returnvalue_3 _returnvalue_3)
        (Variables|/Game/MS/Blueprint/BP_EnemyBoss.BP_EnemyBoss_C|SetIsDead _asbp_enemy_boss true)
        (Default|EnemyDeath _asbp_enemy_boss (Transformation|GetActorLocation _asbp_enemy_boss))
        (Audio|PlaySound2D "/Game/MS/Sound/monster-roar-131214.monster-roar-131214" 0.4 1.0 0.0 0 0)
        (Actor|DestroyActor)
        (else
          (Actor|DestroyActor))))))

(fn ConstructionScript)

(fn Translate
  (params (Direction :type Vector) (Speed :type Float%20%28double-precision%29))
  ;[1 1 1] P = P0 + velocity(dir*speed)*deltaSecond
  (Transformation|SetActorLocation (+ (Transformation|GetActorLocation) (* Direction Speed (Utilities|Time|GetWorldDeltaSeconds))) true false))