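; Boss enemy factory that periodically spawns BP_EnemyBoss once the player reaches level 4.
; On BeginPlay it caches all BP_Spawn actors as candidate spawn points.
; Tick accumulates time up to DelayTime (15 seconds per the comment), then checks BP_Player's level and spawns at a random point.
; The timer resets only on a spawn, so an overdue boss appears as soon as the level requirement is met.
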(event EventBeginPlay
  ;[1 1 1] 스폰 위치 배열에 저장
  (bind _outactors (Actor|GetAllActorsOfClass "/Game/MS/Blueprint/BP_Spawn.BP_Spawn_C"))
  (Variables|Default|SetSpawnList _outactors))

(event Collision|EventActorBeginOverlap
  (params (OtherActor :type Actor%20Object%20Reference)))

(event EventTick
  (params (DeltaSeconds :type Float%20%28single-precision%29))
  (bind _spawnlist (Variables|Default|GetSpawnList))
  ;[1 1 1] 레벨이 4 이상이면 15초마다 보스 생성
  (bind _output_get (Variables|Default|SetCurrentTime (+ (Utilities|Time|GetWorldDeltaSeconds) (Variables|Default|GetCurrentTime))))
  (if (>= _output_get (Variables|Default|GetDelayTime))
    (bind _returnvalue (Actor|GetActorOfClass "/Game/EB/Blueprints/BP_Player.BP_Player_C"))
    (if (>= (Variables|/Game/EB/Blueprints/BP_Player.BP_Player_C|GetPlayerLevel _returnvalue) 4)
      (Game|SpawnActorfromClass "/Game/MS/Blueprint/BP_EnemyBoss.BP_EnemyBoss_C" (Transformation|GetWorldTransform (Variables|/Script/Engine.Actor|GetRootComponent (Utilities|Array|Get(acopy) _spawnlist (Math|Random|RandomInteger (Utilities|Array|Length _spawnlist))))) "Undefined" "MultiplyWithRoot" 0 0)
      (Variables|Default|SetCurrentTime 0.0))))

(fn ConstructionScript)