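; BP_LevelManager is an actor that speeds up enemy spawning as the player levels up.
; Each Tick it finds BP_Player by class and compares its PlayerLevel with the stored LevelCheck.
; When the level is higher, it finds BP_EnemyFactory and cuts its DelayTime by a fixed step while that stays above a floor threshold.
; LevelCheck increments only when a cut is applied.
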(event EventBeginPlay)

(event Collision|EventActorBeginOverlap
  (params (OtherActor :type Actor%20Object%20Reference)))

(event EventTick
  (params (DeltaSeconds :type Float%20%28single-precision%29))
  ;[1 1 1] player level이 level check보다 커지면 스폰 속도(delay time)을 -0.3 씩 감소
  (bind _returnvalue (Actor|GetActorOfClass "/Game/EB/Blueprints/BP_Player.BP_Player_C"))
  (if (> (Variables|/Game/EB/Blueprints/BP_Player.BP_Player_C|GetPlayerLevel _returnvalue) (Variables|Default|GetLevelCheck))
    (bind _returnvalue_2 (Actor|GetActorOfClass "/Game/MS/Blueprint/BP_EnemyFactory.BP_EnemyFactory_C"))
    (if (> (Variables|/Game/MS/Blueprint/BP_EnemyFactory.BP_EnemyFactory_C|GetDelayTime _returnvalue_2) 0.4)
      (Variables|/Game/MS/Blueprint/BP_EnemyFactory.BP_EnemyFactory_C|SetDelayTime _returnvalue_2 (- (Variables|/Game/MS/Blueprint/BP_EnemyFactory.BP_EnemyFactory_C|GetDelayTime _returnvalue_2) 0.3))
      (Variables|Default|SetLevelCheck (+ (Variables|Default|GetLevelCheck) 1)))))

(fn ConstructionScript)