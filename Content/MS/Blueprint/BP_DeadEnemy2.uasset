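; BP_DeadEnemy2 is a short-lived dead-enemy actor that stands in for BP_Enemy2.
; On BeginPlay it turns to face the player pawn, waits briefly, drops an item, spawns the NS_Destroy Niagara effect at its location and destroys itself.
; The drop borrows DropItem from whichever BP_Enemy2 GetActorOfClass finds in the level, passing this actor's location, with no validity check.
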(event EventBeginPlay
  (bind _returnvalue (Transformation|GetActorLocation))
  (Transformation|SetActorRotation (Math|Rotator|FindLookatRotation (Transformation|GetActorLocation) (Transformation|GetActorLocation (Game|Player|GetPlayerPawn 0))))
  (Utilities|FlowControl|Delay 2.5)
  (bind _returnvalue_2 (Actor|GetActorOfClass "/Game/EB/Blueprints/BP_Enemy2.BP_Enemy2_C"))
  (Default|DropItem _returnvalue_2 _returnvalue)
  (Niagara|SpawnSystematLocation "/Game/MS/Particle/NS_Destroy.NS_Destroy" _returnvalue)
  (Actor|DestroyActor))

(event Collision|EventActorBeginOverlap
  (params (OtherActor :type Actor%20Object%20Reference)))

(event EventTick
  (params (DeltaSeconds :type Float%20%28single-precision%29)))

(fn ConstructionScript)