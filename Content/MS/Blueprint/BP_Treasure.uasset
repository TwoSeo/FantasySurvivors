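; BP_Treasure is a treasure pickup that triggers a reward screen when the player overlaps it.
; On overlap with BP_Player it spawns a coin-burst Niagara effect at the player and waits a second.
; It then pauses the game, shows the WBP_Treasure widget with the mouse cursor, resets CurrentTime and plays a 2D coin sound.
; A UI-only input mode call is present but unconnected.
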(event EventBeginPlay)

(event Collision|EventActorBeginOverlap
  (params (OtherActor :type Actor%20Object%20Reference))
  (Utilities|Casting|CastToBP_Player OtherActor)
  (Niagara|SpawnSystematLocation "/Game/sA_PickupSet_1/Fx/NiagaraSystems/NS_CoinBurst.NS_CoinBurst" (Transformation|GetActorLocation OtherActor) "0, 0, 0" "10.000000,10.000000,10.000000")
  (Utilities|FlowControl|Delay 1.0)
  (Game|SetGamePaused true)
  (bind _returnvalue (UserInterface|CreateWidget "/Game/MS/UI/WBP_Treasure.WBP_Treasure_C"))
  (UserInterface|Viewport|AddtoViewport _returnvalue 0)
  (Variables|/Script/Engine.PlayerController|SetbShowMouseCursor (Game|GetPlayerController 0) true) ; 마우스 커서 보이기
  (Variables|Default|SetcurrentTime 0.0)
  (Audio|PlaySound2D "/Game/MS/Sound/Game-Score-Glitch-Coin.Game-Score-Glitch-Coin" 0.4 1.0 0.0 0 0))

(event EventTick
  (params (DeltaSeconds :type Float%20%28single-precision%29)))

(fn ConstructionScript)