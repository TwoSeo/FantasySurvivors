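; BP_EnemyFactory is an enemy spawner that also starts the background music when play begins.
; On BeginPlay it caches every BP_Spawn actor as a spawn point.
; Tick accumulates delta time and, once DelayTime passes, spawns an enemy at a random spawn point and resets the timer.
; BP_Player's PlayerLevel selects the pool: only BP_Enemy at level 1 or below, otherwise a random pick between BP_Enemy and BP_Enemy2.
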(event EventBeginPlay
  (bind _outactors (Actor|GetAllActorsOfClass "/Game/MS/Blueprint/BP_Spawn.BP_Spawn_C"))
  (Variables|Default|SetSpawnList _outactors) ; 스폰위치 배열에 저장
  (Audio|PlaySound2D "/Game/MS/Sound/alexander-nakarada-the-great-battle_chosic_com_.alexander-nakarada-the-great-battle_chosic_com_" 0.3 1.0 0.0 0 0))

(event Collision|EventActorBeginOverlap
  (params (OtherActor :type Actor%20Object%20Reference)))

(event EventTick
  (params (DeltaSeconds :type Float%20%28single-precision%29))
  (bind _spawnlist (Variables|Default|GetSpawnList))
  (bind _returnvalue (Utilities|Array|Length _spawnlist))
  (bind _returnvalue_2 (Math|Random|RandomInteger _returnvalue))
  (bind _output (Utilities|Array|Get(acopy) _spawnlist _returnvalue_2))
  (bind _rootcomponent (Variables|/Script/Engine.Actor|GetRootComponent _output))
  (bind _returnvalue_3 (Transformation|GetWorldTransform _rootcomponent))
  (bind _output_get (Variables|Default|SetCurrentTime (+ (Utilities|Time|GetWorldDeltaSeconds) (Variables|Default|GetCurrentTime))))
  (if (>= _output_get (Variables|Default|GetDelayTime))
    (bind _returnvalue_4 (Actor|GetActorOfClass "/Game/EB/Blueprints/BP_Player.BP_Player_C"))
    (if (<= (Variables|/Game/EB/Blueprints/BP_Player.BP_Player_C|GetPlayerLevel _returnvalue_4) 1)
      (Game|SpawnActorfromClass "/Game/EB/Blueprints/BP_Enemy.BP_Enemy_C" _returnvalue_3 "AdjustIfPossibleButAlwaysSpawn" "MultiplyWithRoot" 0 0)
      (Variables|Default|SetCurrentTime 0.0)
      (else
        (bind _output_get_2 (Variables|Default|SetRandomEnemy (Math|Random|RandomInteger 2)))
        (switch int _output_get_2
          (:0
            (Game|SpawnActorfromClass "/Game/EB/Blueprints/BP_Enemy.BP_Enemy_C" _returnvalue_3 "AdjustIfPossibleButAlwaysSpawn" "MultiplyWithRoot" 0 0)
            (Variables|Default|SetCurrentTime 0.0))
          (:1
            (Game|SpawnActorfromClass "/Game/EB/Blueprints/BP_Enemy2.BP_Enemy2_C" _returnvalue_3 "AdjustIfPossibleButAlwaysSpawn" "MultiplyWithRoot" 0 0)
            (Variables|Default|SetCurrentTime 0.0)))))))

(fn ConstructionScript)